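; LevelExit is a level exit actor that activates once the game instance reports that all keys are found.
; Every Tick it polls that AllKeysFound flag on NewGameInstance to toggle the particle effect and swap the sphere's material.
; When a ThirdPersonCharacter overlaps Sphere1 with the flag set, it creates the LevelClear widget and adds it to the viewport.
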(event OnComponentBeginOverlap(Sphere1)
  (params (OverlappedComponent :type Primitive%20Component%20Object%20Reference) (OtherActor :type Actor%20Object%20Reference) (OtherComp :type Primitive%20Component%20Object%20Reference) (OtherBodyIndex :type Integer) (bFromSweep :type Boolean) (SweepResult :type Hit%20Result%20Structure%20%28by%20ref%29))
  (Utilities|Casting|CastToThirdPersonCharacter OtherActor)
  (bind _asnew_game_instance (Utilities|Casting|CastToNewGameInstance (Game|GetGameInstance)))
  (if (Variables|/Game/NewGameInstance.NewGameInstance_C|GetAllKeysFound _asnew_game_instance)
    (bind _returnvalue (UserInterface|CreateWidget "/Game/PlatformGame/LukeH/Widgets/LevelClear.LevelClear_C" (Game|GetPlayerController 0)))
    (UserInterface|Viewport|AddtoViewport _returnvalue 0)))

(event EventBeginPlay)

(event Collision|EventActorBeginOverlap
  (params (OtherActor :type Actor%20Object%20Reference)))

(event EventTick
  (params (DeltaSeconds :type Float%20%28single-precision%29))
  (bind _asnew_game_instance (Utilities|Casting|CastToNewGameInstance (Game|GetGameInstance)))
  (if (Variables|/Game/NewGameInstance.NewGameInstance_C|GetAllKeysFound _asnew_game_instance)
    (Rendering|SetVisibility (Variables|Default|GetParticleSystem) true false)
    (Rendering|Material|SetMaterial (Variables|Default|GetSphere) 0 "/Game/StarterContent/Materials/M_Wood_Pine.M_Wood_Pine")
    (else
      (Rendering|SetVisibility (Variables|Default|GetParticleSystem) false false)
      (Rendering|Material|SetMaterial (Variables|Default|GetSphere) 0 "/Game/StarterContent/Materials/M_Basic_Floor.M_Basic_Floor"))))

(fn ConstructionScript)