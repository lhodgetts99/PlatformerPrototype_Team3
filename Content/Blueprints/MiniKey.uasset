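; MiniKey is a spinning collectible key pickup that the third-person character picks up by overlapping it.
; On overlap it destroys itself and increments the TotalMiniKeys count on NewGameInstance.
; It applies its Colour material to the mesh at BeginPlay and rotates around yaw each tick at SpinSpeed, scaled by delta time.
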(event EventBeginPlay
  (Rendering|Material|SetMaterial (Variables|Default|GetStaticMesh) 0 (Variables|Colour|GetColour)))

(event Collision|EventActorBeginOverlap
  (params (OtherActor :type Actor%20Object%20Reference))
  (Utilities|Casting|CastToThirdPersonCharacter OtherActor)
  (Actor|DestroyActor)
  (bind _asnew_game_instance (Utilities|Casting|CastToNewGameInstance (Game|GetGameInstance)))
  (Variables|/Game/NewGameInstance.NewGameInstance_C|SetTotalMiniKeys _asnew_game_instance (+ (Variables|/Game/NewGameInstance.NewGameInstance_C|GetTotalMiniKeys _asnew_game_instance) 1)))

(event EventTick
  (params (DeltaSeconds :type Float%20%28single-precision%29))
  (Transformation|AddActorLocalRotation (Math|Rotator|MakeRotator 0.0 0.0 (* DeltaSeconds (Variables|Default|GetSpinSpeed))) false false))

(fn ConstructionScript)