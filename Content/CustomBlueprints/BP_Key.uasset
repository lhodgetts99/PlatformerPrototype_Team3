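; BP_Key is a collectible key pickup that spins around its yaw axis every tick at SpinSpeed.
; When a ThirdPersonCharacter overlaps it, the key destroys itself and increments that character's KeyCount.
; It also increments TotalKeysFoundRecord on NewGameInstance and fires the CallEvent dispatcher.
; When the character's count equals the game instance's KeyTarget, it sets AllKeysFound there.
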(event EventBeginPlay)

(event Collision|EventActorBeginOverlap
  (params (OtherActor :type Actor%20Object%20Reference))
  (bind _asthird_person_character (Utilities|Casting|CastToThirdPersonCharacter OtherActor))
  (Actor|DestroyActor)
  (Variables|/Game/ThirdPersonBP/Blueprints/ThirdPersonCharacter.ThirdPersonCharacter_C|SetKeyCount _asthird_person_character (+ (Variables|/Game/ThirdPersonBP/Blueprints/ThirdPersonCharacter.ThirdPersonCharacter_C|GetKeyCount _asthird_person_character) 1))
  (bind _asnew_game_instance (Utilities|Casting|CastToNewGameInstance (Game|GetGameInstance)))
  (Variables|/Game/NewGameInstance.NewGameInstance_C|SetTotalKeysFoundRecord _asnew_game_instance (+ (Variables|/Game/NewGameInstance.NewGameInstance_C|GetTotalKeysFoundRecord _asnew_game_instance) 1))
  (Default|CallCallEvent)
  (if (== (Variables|/Game/NewGameInstance.NewGameInstance_C|GetKeyTarget _asnew_game_instance) (Variables|/Game/ThirdPersonBP/Blueprints/ThirdPersonCharacter.ThirdPersonCharacter_C|GetKeyCount _asthird_person_character))
    (Variables|/Game/NewGameInstance.NewGameInstance_C|SetAllKeysFound _asnew_game_instance true)))

(event EventTick
  (params (DeltaSeconds :type Float%20%28single-precision%29))
  (Transformation|AddActorLocalRotation (Math|Rotator|MakeRotator 0.0 0.0 (* DeltaSeconds (Variables|Default|GetSpinSpeed))) false false))

(fn ConstructionScript)